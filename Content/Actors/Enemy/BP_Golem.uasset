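; BP_Golem is an enemy that senses the player, attacks, and completes quests targeting it when killed, notifying matching NPCs.
; Pawn sensing sets the hasSeenPlayer blackboard key, clearing it after a retriggerable delay.
; AttdackPlayer randomly starts a punch or slam through the AnimBP; punch traces apply damage and time-dilation hitstop only when the player's IsDodging is true.
; A separate AttackPlayer event uses a forward sphere trace, montage and ApplyDamage.
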(event OnItemAdded(DidItHitActor)
  (params (LastItem :type Hit%20Result%20Structure))
  (bind _hitstopduration (Variables|Default|GetHitstopDuration))
  (bind _asthird_person_character (Utilities|Casting|CastToThirdPersonCharacter (.HitActor (Collision|BreakHitResult LastItem))))
  (if (Variables|/Game/ThirdPersonBP/Blueprints/ThirdPersonCharacter.ThirdPersonCharacter_C|GetbIsDodging _asthird_person_character)
    (Default|AffectHealth _asthird_person_character (Variables|Default|GetDamage))
    (Default|StartHitstop _asthird_person_character _hitstopduration)
    (CallFunction|StartHitstop _hitstopduration)))

(event OnSeePawn(PawnSensing)
  (params (Pawn :type Pawn%20Object%20Reference))
  (Utilities|FlowControl|Sequence
    (:then_0
      (Utilities|Casting|CastToThirdPersonCharacter Pawn)
      (AI|Components|Blackboard|SetValueasBool (AI|GetBlackboard (AI|GetAIController self)) (Utilities|Name|MakeLiteralName "hasSeenPlayer") true))
    (:then_1
      (Utilities|FlowControl|RetriggerableDelay 3.0)
      (AI|Components|Blackboard|SetValueasBool (AI|GetBlackboard (AI|GetAIController self)) (Utilities|Name|MakeLiteralName "hasSeenPlayer") false))))

(event Custom|UpdateIsDead
  ;[1 1 1] Vérifie si le personnage n'as plus de point de vie
  (if (<= (Variables|State|GetHealthPoint) 0.0)
    (Utilities|FlowControl|Sequence
      (:then_0
        (bind _asthird_person_character (Utilities|Casting|CastToThirdPersonCharacter (Pawn|GetControlledPawn (Game|GetPlayerController 0))))
        (for _array_element (Variables|/Game/ThirdPersonBP/Blueprints/ThirdPersonCharacter.ThirdPersonCharacter_C|GetActiveQuests _asthird_person_character)
          (if (== self (.actorreference (Variables|/Game/BP_Quest.BP_Quest_C|GetQuestInfo _array_element)))
            (Default|QuestComplete _asthird_person_character _array_element)
            (bind _outactors (Actor|GetAllActorsOfClass "/Game/Actors/NPCs/BP_NPC.BP_NPC_C"))
            (for _array_element_2 _outactors
              (if (Utilities|Enum|Equal(Enum) (.questname (Variables|/Game/BP_Quest.BP_Quest_C|GetQuestInfo _array_element)) (.questname (Variables|/Game/Actors/NPCs/BP_NPC.BP_NPC_C|GetQuestReference _array_element_2)))
                (Default|EventQuestComplete _array_element_2))))))
      (:then_1
        (Actor|DestroyActor)))))

(event Custom|Attack%20Player
  (bind _returnvalue (Transformation|GetActorLocation))
  (bind (_outhit _returnvalue_2) (Collision|SphereTraceForObjects _returnvalue (+ _returnvalue (* (Math|Vector|GetForwardVector (Transformation|GetActorRotation)) 2.5e+02)) 1.2e+02 (Utilities|Array|MakeArray "ObjectTypeQuery3") false 0 "ForDuration"))
  (if _returnvalue_2
    (Utilities|Casting|CastToThirdPersonCharacter (.HitActor (Collision|BreakHitResult _outhit)))
    (Animation|PlayAnimMontage "/Game/Actors/Enemy/Golem_Punch_Montage.Golem_Punch_Montage" 1.0 "None")
    (Game|Damage|ApplyDamage (.HitActor (Collision|BreakHitResult _outhit)) 1e+01 0 0)
    (Development|PrintString "DAMAGED")))

(event EventEndHitstop
  (Variables|Default|SetCustomTimeDilation 1.0))

(event EventAffectHealth
  (params (Delta :type Float%20%28double-precision%29))
  ;[1 1 1] modifier les points de vie
  (Variables|State|SetHealthPoint (+ Delta (Variables|State|GetHealthPoint)))
  (CallFunction|UpdateIsDead))

(event EventStartHitstop
  (params (Length :type Float%20%28double-precision%29))
  (Variables|Default|SetCustomTimeDilation 0.15)
  (Utilities|Time|SetTimerbyEvent (delegate EventEndHitstop) Length))

(fn ConstructionScript
  (Class|DidItHitActorComponent|SetupVariables (Variables|Default|GetDidItHitActor) (Variables|Default|GetHiddenStaticSocket)))

(fn UpdateHealthPoint
  (params (Delta :type Float%20%28double-precision%29))
  ;[1 1 1] Met à jours les points de vie
)

(fn AttdackPlayer
  (params (AttackBTTask :type BT%20Task%20Blueprint%20Base%20Object%20Reference))
  (bind _anim_bp_golem (Variables|State|GetAnim%20BP%20Golem))
  (Variables|State|SetAttackBTTask AttackBTTask)
  (if (Math|Random|RandomBool)
    (Variables|/Game/Actors/Enemy/AnimBP_Golem.AnimBP_Golem_C|SetStartPunch _anim_bp_golem true)
    (Class|DidItHitActorComponent|ToggleTraceCheck (Variables|Default|GetDidItHitActor) true)
    (else
      (Variables|/Game/Actors/Enemy/AnimBP_Golem.AnimBP_Golem_C|SetStartSlam _anim_bp_golem true))))

(fn ActivateSlam
  (CallFunction|EndBTTask))

(fn EndPunchHitbox
  (Class|DidItHitActorComponent|ToggleTraceCheck (Variables|Default|GetDidItHitActor) false)
  (CallFunction|EndBTTask))

(fn EndBTTask)