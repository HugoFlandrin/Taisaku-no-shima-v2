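; Kitsune enemy that runs a behavior tree through its AIC_Kitsune controller and attacks by spawning fireballs.
; AffectHealth and UpdateHealthPoint add a delta to health, then destroy the actor at zero or below.
; StartHitstop briefly slows the actor with custom time dilation until a timer restores it.
; AttackPlayer spawns Fire_Ball at SpawnProjectile's transform; its forward trace result and Player input go unused.
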(event Custom|UpdateIsDead
  ;[1 1 1] Vérifie si le personnage n'as plus de point de vie
  (if (<= (Variables|State|GetHealthPoint) 0.0)
    (Actor|DestroyActor)))

(event EventAffectHealth
  (params (Delta :type Float%20%28double-precision%29))
  (Variables|State|SetHealthPoint (+ Delta (Variables|State|GetHealthPoint)))
  (CallFunction|UpdateIsDead))

(event EventStartHitstop
  (params (Length :type Float%20%28double-precision%29))
  (Variables|Default|SetCustomTimeDilation 0.15)
  (Utilities|Time|SetTimerbyEvent (delegate EventEndHitstop) Length))

(event EventEndHitstop
  (Variables|Default|SetCustomTimeDilation 1.0))

(event EventBeginPlay
  (bind _asaic_kitsune (Utilities|Casting|CastToAIC_Kitsune (AI|GetAIController self)))
  (bind _output_get (Variables|Default|SetAIController _asaic_kitsune))
  (Default|RunBehaviorTree _output_get))

(fn ConstructionScript
  (CallFunction|UpdateHealthPoint 0.0))

(fn UpdateHealthPoint
  (params (Delta :type Float%20%28double-precision%29))
  ;[1 1 1] Met à jours les points de vie
  (bind _output_get (Variables|State|SetHealthPoint (+ Delta (Variables|State|GetHealthPoint))))
  (CallFunction|UpdateIsDead)
  (return _output_get))

(fn AttackPlayer
  (params (Player :type Actor%20Object%20Reference))
  (bind _returnvalue (Transformation|GetActorLocation))
  (Collision|LineTraceByChannel _returnvalue (+ _returnvalue (* (Transformation|GetActorForwardVector) "300.000000,300.000000,300.000000")) "TraceTypeQuery1" false 0 "None" true "(R=1.000000,G=0.000000,B=0.000000,A=1.000000)" "(R=0.000000,G=1.000000,B=0.000000,A=1.000000)" 2.0)
  (Game|SpawnActorfromClass "/Game/Actors/Enemy/Fire_Ball.Fire_Ball_C" (Transformation|GetWorldTransform (Variables|Default|GetSpawnProjectile)) "Undefined" "OverrideRootScale" 0 0))