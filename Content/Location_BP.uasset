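; Location_BP is a trigger volume that completes quests whose objective is reaching that location.
; When the player's ThirdPersonCharacter overlaps the Box, it checks each active quest for an ActorReference pointing to this actor and calls QuestComplete on matches.
; It then scans all BP_NPC actors and fires EventQuestComplete on those whose quest name matches the completed quest.
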(event OnComponentBeginOverlap(Box)
  (params (OverlappedComponent :type Primitive%20Component%20Object%20Reference) (OtherActor :type Actor%20Object%20Reference) (OtherComp :type Primitive%20Component%20Object%20Reference) (OtherBodyIndex :type Integer) (bFromSweep :type Boolean) (SweepResult :type Hit%20Result%20Structure%20%28by%20ref%29))
  (bind _asthird_person_character (Utilities|Casting|CastToThirdPersonCharacter OtherActor))
  (for _array_element (Variables|/Game/ThirdPersonBP/Blueprints/ThirdPersonCharacter.ThirdPersonCharacter_C|GetActiveQuests _asthird_person_character)
    (if (== self (.actorreference (Variables|/Game/BP_Quest.BP_Quest_C|GetQuestInfo _array_element)))
      (Default|QuestComplete _asthird_person_character _array_element)
      (bind _outactors (Actor|GetAllActorsOfClass "/Game/Actors/NPCs/BP_NPC.BP_NPC_C"))
      (for _array_element_2 _outactors
        (if (Utilities|Enum|Equal(Enum) (.questname (Variables|/Game/BP_Quest.BP_Quest_C|GetQuestInfo _array_element)) (.questname (Variables|/Game/Actors/NPCs/BP_NPC.BP_NPC_C|GetQuestReference _array_element_2)))
          (Default|EventQuestComplete _array_element_2))))))

(fn ConstructionScript)